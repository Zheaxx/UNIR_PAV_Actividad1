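; BP_SS_PowerUpMultiShot is a power-up that toggles multi-shot on the player character.
; ExecutePowerUp calls EnableMultiShot on the passed character, and EndPowerUp calls DisableMultiShot, with both printing debug strings.
; The validity check in ExecutePowerUp runs after the enable call, so it only selects which message prints.
; The event graph holds only disabled default events, and the construction script just calls its parent.
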(event EventBeginPlay
  (|CallParentFunction) ; This node is disabled and will not be called.\nDrag off pins to build functionality.
)

(event Collision|EventActorBeginOverlap
  (params (OtherActor :type Actor%20Object%20Reference))
  (|CallParentFunction OtherActor) ; This node is disabled and will not be called.\nDrag off pins to build functionality.
)

(event EventTick
  (params (DeltaSeconds :type Float%20%28single-precision%29))
  (|CallParentFunction DeltaSeconds) ; This node is disabled and will not be called.\nDrag off pins to build functionality.
)

(fn ConstructionScript
  (|CallParentFunction))

(fn ExecutePowerUp
  (params (_PlayerCharacter :type BP%20SS%20Player%20Character%20Object%20Reference))
  (Default|EnableMultiShot _PlayerCharacter)
  (Utilities|IsValid _PlayerCharacter
    (:Is%20Valid
      (Development|PrintString "ENABLED MULTI SHOT"))
    (:Is%20Not%20Valid
      (Development|PrintString "PLAYER NOT VALID"))))

(fn EndPowerUp
  (params (_PlayerCharacter :type BP%20SS%20Player%20Character%20Object%20Reference))
  (Development|PrintString "MULTI SHOT DISABLED" true true "(R=0.000000,G=1.000000,B=0.268016,A=1.000000)")
  (Default|DisableMultiShot _PlayerCharacter))