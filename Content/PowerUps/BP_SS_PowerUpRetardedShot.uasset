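; Power-up Blueprint that gives the player character a large temporary speed boost, despite the "Shot" in its asset name.
; ExecutePowerUp sets movement speed to a fixed multiple of the character's DefaultMaxSpeed, and EndPowerUp restores that default.
; The event graph holds only disabled stubs and the construction script just calls its parent, so timing and triggering are not handled here.
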(event EventBeginPlay
  (|CallParentFunction) ; This node is disabled and will not be called.\nDrag off pins to build functionality.
)

(event Collision|EventActorBeginOverlap
  (params (OtherActor :type Actor%20Object%20Reference))
  (|CallParentFunction OtherActor) ; This node is disabled and will not be called.\nDrag off pins to build functionality.
)

(event EventTick
  (params (DeltaSeconds :type Float%20%28single-precision%29))
  (|CallParentFunction DeltaSeconds) ; This node is disabled and will not be called.\nDrag off pins to build functionality.
)

(fn ConstructionScript
  (|CallParentFunction))

(fn ExecutePowerUp
  (params (_PlayerCharacter :type BP%20SS%20Player%20Character%20Object%20Reference))
  (Default|SetMovementSpeed _PlayerCharacter (* (Variables|/Game/Players/BP_SS_PlayerCharacter.BP_SS_PlayerCharacter_C|GetDefaultMaxSpeed _PlayerCharacter) 5.0)))

(fn EndPowerUp
  (params (_PlayerCharacter :type BP%20SS%20Player%20Character%20Object%20Reference))
  (Default|SetMovementSpeed _PlayerCharacter (Variables|/Game/Players/BP_SS_PlayerCharacter.BP_SS_PlayerCharacter_C|GetDefaultMaxSpeed _PlayerCharacter)))