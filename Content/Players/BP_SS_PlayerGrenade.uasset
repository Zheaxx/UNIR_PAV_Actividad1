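; BP_SS_PlayerGrenade is a player grenade that explodes on a random timer of a few seconds after BeginPlay.
; On explosion it switches its capsule to overlap-all with overlap events enabled, then spawns a scaled-up explosion emitter and plays a 2D sound.
; A brief delay keeps that overlap active before the actor destroys itself.
; The blueprint applies no damage and handles no overlaps itself.
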(event Custom|Explode
  (bind _capsule (Variables|Default|GetCapsule))
  (Variables|/Script/Engine.PrimitiveComponent|SetbGenerateOverlapEvents _capsule true)
  (Collision|SetCollisionProfileName _capsule "OverlapAllDynamic" true :!class /Script/Engine.PrimitiveComponent)
  (Effects|SpawnEmitteratLocation "/Game/StarterContent/Particles/P_Explosion.P_Explosion" (Transformation|GetActorLocation) "0, 0, 0" "5.000000,5.000000,5.000000")
  (Audio|PlaySound2D "/Engine/VREditor/Sounds/UI/Enter_Play.Enter_Play" 1.0 1.0 0.0 0 0)
  (Utilities|FlowControl|Delay 0.2)
  (Actor|DestroyActor))

(event EventBeginPlay
  (|CallParentFunction)
  (bind _output_get (Variables|Default|SetTimeToExplode (Math|Random|RandomFloatinRange 2.0 6.0)))
  (Utilities|Time|SetTimerbyEvent (delegate Custom|Explode) _output_get))

(event EventTick
  (params (DeltaSeconds :type Float%20%28single-precision%29))
  (|CallParentFunction DeltaSeconds) ; This node is disabled and will not be called.\nDrag off pins to build functionality.
)

(fn ConstructionScript
  (|CallParentFunction))