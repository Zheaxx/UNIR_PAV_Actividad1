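; Player character for a shooter that moves via Enhanced Input, fires on a timer-gated cooldown and takes damage from enemy-tagged overlaps.
; Damage drains the spinning shield while it is up, otherwise lives, and the game mode is notified of shield, life and death changes.
; Power-up functions toggle the shield with a larger collision radius, three-point multishot and grenade ammo, add clamped lives, or set movement speed.
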(event Custom|UpdateFire
  (Variables|Default|SetCanFire true))

(event Custom|TakeDamage
  (params (DamageToTake :type Integer))
  (if (Variables|Default|GetIsShieldEnabled)
    (CallFunction|SubstractShield DamageToTake)
    (else
      (CallFunction|SubstractLifes DamageToTake))))

(event Input|EnhancedActionEvents|EnhancedInputActionIA_Movement
  (params (ActionValue :type Vector%202D%20Structure) (ElapsedSeconds :type Float%20%28double-precision%29) (TriggeredSeconds :type Float%20%28double-precision%29) (InputAction :type Input%20Action%20Object%20Reference :default "/Game/Input/IA_Movement.IA_Movement"))
  (Pawn|Input|AddMovementInput (Transformation|GetActorRightVector) (.x ActionValue) false)
  (Pawn|Input|AddMovementInput (Transformation|GetActorForwardVector) (.y ActionValue) false))

(event Input|EnhancedActionEvents|EnhancedInputActionIA_Fire
  (params (ActionValue :type Boolean) (ElapsedSeconds :type Float%20%28double-precision%29) (TriggeredSeconds :type Float%20%28double-precision%29) (InputAction :type Input%20Action%20Object%20Reference :default "/Game/Input/IA_Fire.IA_Fire"))
  (if (Variables|Default|GetCanFire)
    (CallFunction|DoFire)
    (Variables|Default|SetCanFire false)
    (Utilities|Time|SetTimerbyEvent (delegate Custom|UpdateFire) (Variables|Default|GetFireDelay))))

(event EventBeginPlay
  (bind _asplayer_controller (Utilities|Casting|CastToPlayerController (Pawn|GetController)))
  (Utilities|IsValid (PlayerController|LocalPlayerSubsystems|GetEnhancedInputLocalPlayerSubsystem _asplayer_controller)
    (:Is%20Valid
      (Input|AddMappingContext (PlayerController|LocalPlayerSubsystems|GetEnhancedInputLocalPlayerSubsystem _asplayer_controller) "/Game/Input/IMC_Mapping.IMC_Mapping" 0 "(bIgnoreAllPressedKeysUntilRelease=True,bForceImmediately=False,bNotifyUserSettings=False)")
      (Variables|Default|SetDefaultMaxSpeed (Class|MovementComponent|GetMaxSpeed (Variables|Character|GetCharacterMovement)))
      (Rendering|SetVisibility (Variables|Default|GetShieldSceneCmp) (Variables|Default|GetIsShieldEnabled) true)
      (bind _asbp_ss_game_mode (Utilities|Casting|CastToBP_SS_GameMode (Game|GetGameMode)))
      (Variables|Default|Set_GameMode _asbp_ss_game_mode))))

(event Collision|EventActorBeginOverlap
  (params (OtherActor :type Actor%20Object%20Reference))
  (if (Utilities|Array|ContainsItem (Variables|/Script/Engine.Actor|GetTags OtherActor) (Variables|Default|GetEnemyTag))
    (bind _asbp_ss_enemy_ammo (Utilities|Casting|CastToBP_SS_EnemyAmmo OtherActor)
      (:then
        (CallFunction|TakeDamage (Variables|/Game/Enemies/BP_SS_EnemyAmmo.BP_SS_EnemyAmmo_C|GetDamage _asbp_ss_enemy_ammo)))
      (:CastFailed
        (CallFunction|TakeDamage 1)))))

(event EventTick
  (params (DeltaSeconds :type Float%20%28single-precision%29))
  (if (Variables|Default|GetIsShieldEnabled)
    (Transformation|AddLocalRotation (Variables|Default|GetShieldSceneCmp) "0.000000,3.000000,0.000000" false false)))

(fn ConstructionScript)

(fn DoFire
  (bind _ammo (Variables|Default|GetAmmo))
  (Game|SpawnActorfromClass (Variables|Default|GetAmmo) (Transformation|GetWorldTransform (Variables|Default|GetFirePoint)) "Undefined" "MultiplyWithRoot" 0 0)
  (if (Variables|Default|GetIsMultiShotEnabled)
    (Utilities|FlowControl|Sequence
      (:then_0
        (Game|SpawnActorfromClass _ammo (Transformation|GetWorldTransform (Variables|Default|GetFirePoint2)) "Undefined" "MultiplyWithRoot" 0 0))
      (:then_1
        (Game|SpawnActorfromClass _ammo (Transformation|GetWorldTransform (Variables|Default|GetFirePoint3)) "Undefined" "MultiplyWithRoot" 0 0)))))

(fn SetMovementSpeed
  (params (NewMovementSpeed :type Float%20%28double-precision%29))
  (Variables|/Script/Engine.CharacterMovementComponent|SetMaxWalkSpeed (Variables|Character|GetCharacterMovement) NewMovementSpeed))

(fn EnableShield
  (bind __gamemode (Variables|Default|Get_GameMode))
  (Variables|Default|SetShields 3)
  (Rendering|SetVisibility (Variables|Default|GetShieldSceneCmp) true true)
  (Components|Sphere|SetSphereRadius (Variables|Default|GetMainCapsule) 195.0 true)
  (Variables|Default|SetIsShieldEnabled true)
  (Utilities|IsValid __gamemode
    (:Is%20Valid
      (Default|ShieldEnabled __gamemode))
    (:Is%20Not%20Valid
      (Development|PrintString "ERROR --> Enable shield: Game Mode is null" true true "(R=1.000000,G=0.000000,B=0.000000,A=1.000000)"))))

(fn DisableShield
  (bind __gamemode (Variables|Default|Get_GameMode))
  (Variables|Default|SetShields 0)
  (Rendering|SetVisibility (Variables|Default|GetShieldSceneCmp) false true)
  (Components|Sphere|SetSphereRadius (Variables|Default|GetMainCapsule) 7e+01 true)
  (Variables|Default|SetIsShieldEnabled false)
  (Utilities|IsValid __gamemode
    (:Is%20Valid
      (Default|ShieldDisabled __gamemode))
    (:Is%20Not%20Valid
      (Development|PrintString "ERROR --> Enable shield: Game Mode is null" true true "(R=1.000000,G=0.000000,B=0.000000,A=1.000000)"))))

(fn SubstractLifes
  (params (Lifes :type Integer))
  (bind __gamemode (Variables|Default|Get_GameMode))
  (Variables|Default|SetLifes (- (Variables|Default|GetLifes) Lifes))
  (Utilities|IsValid (Variables|Default|Get_GameMode)
    (:Is%20Valid
      (if (<= (Variables|Default|GetLifes) 0)
        (Default|PlayerDead __gamemode)
        (else
          (Default|TakeLifesDamage __gamemode))))
    (:Is%20Not%20Valid
      (Development|PrintString "ERROR --> Enable shield: Game Mode is null" true true "(R=1.000000,G=0.000000,B=0.000000,A=1.000000)"))))

(fn SubstractShield
  (params (ShieldsToSubstract :type Integer))
  (Variables|Default|SetShields (- (Variables|Default|GetShields) ShieldsToSubstract))
  (Default|TakeShieldDamage (Variables|Default|Get_GameMode))
  (if (<= (Variables|Default|GetShields) 0)
    (CallFunction|DisableShield)))

(fn AddLifes
  (params (LifesToAdd :type Integer))
  (bind __gamemode (Variables|Default|Get_GameMode))
  (Variables|Default|SetLifes (Math|Integer|Clamp(Integer) (+ LifesToAdd (Variables|Default|GetLifes)) 1 3))
  (Utilities|IsValid __gamemode
    (:Is%20Valid
      (Default|HealLife __gamemode))))

(fn EnableMultiShot
  (Variables|Default|SetIsMultiShotEnabled true))

(fn DisableMultiShot
  (Variables|Default|SetIsMultiShotEnabled false))

(fn EnableGrenades
  (Variables|Default|SetAmmo "/Game/Players/BP_SS_PlayerGrenade.BP_SS_PlayerGrenade_C"))

(fn DisableGrenades
  (Variables|Default|SetAmmo "/Game/Players/BP_SS_PlayerAmmo.BP_SS_PlayerAmmo_C"))