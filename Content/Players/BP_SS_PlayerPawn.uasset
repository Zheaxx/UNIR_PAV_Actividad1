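; BP_SS_PlayerPawn is a player pawn that moves through Enhanced Input, with a placeholder fire action.
; BeginPlay adds the IMC_Mapping context to the owning player controller's input subsystem.
; IA_Movement stores its axis value and clears it on completion or cancel; Tick applies it along right and forward vectors, scaled by Speed and delta time, without sweeping.
; IA_Fire only prints a debug string.
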(event Input|EnhancedActionEvents|EnhancedInputActionIA_Fire
  (params (ActionValue :type Boolean) (ElapsedSeconds :type Float%20%28double-precision%29) (TriggeredSeconds :type Float%20%28double-precision%29) (InputAction :type Input%20Action%20Object%20Reference :default "/Game/Input/IA_Fire.IA_Fire"))
  (Development|PrintString "Firing"))

(event Input|EnhancedActionEvents|EnhancedInputActionIA_Movement
  (params (ActionValue :type Vector%202D%20Structure) (ElapsedSeconds :type Float%20%28double-precision%29) (TriggeredSeconds :type Float%20%28double-precision%29) (InputAction :type Input%20Action%20Object%20Reference :default "/Game/Input/IA_Movement.IA_Movement"))
  (:Triggered
    (Variables|Default|SetInputSaved ActionValue))
  (:Canceled
    (Variables|Default|SetInputSaved "" :!label _label))
  (:Completed
    (goto _label)))

(event EventBeginPlay
  (bind _asplayer_controller (Utilities|Casting|CastToPlayerController (Pawn|GetController)))
  (Utilities|IsValid (PlayerController|LocalPlayerSubsystems|GetEnhancedInputLocalPlayerSubsystem _asplayer_controller)
    (:Is%20Valid
      (Input|AddMappingContext (PlayerController|LocalPlayerSubsystems|GetEnhancedInputLocalPlayerSubsystem _asplayer_controller) "/Game/Input/IMC_Mapping.IMC_Mapping" 0 "(bIgnoreAllPressedKeysUntilRelease=True,bForceImmediately=False,bNotifyUserSettings=False)"))))

(event Collision|EventActorBeginOverlap
  (params (OtherActor :type Actor%20Object%20Reference)))

(event EventTick
  (params (DeltaSeconds :type Float%20%28single-precision%29))
  (bind _speed (Variables|Default|GetSpeed))
  (bind _inputsaved (Variables|Default|GetInputSaved))
  (bind _returnvalue (* DeltaSeconds _speed))
  (Transformation|SetActorLocation (+ (Transformation|GetActorLocation) (+ (* (Transformation|GetActorRightVector) (* _returnvalue (.x _inputsaved))) (* (* _returnvalue (.y _inputsaved)) (Transformation|GetActorForwardVector)))) false false))

(fn ConstructionScript)