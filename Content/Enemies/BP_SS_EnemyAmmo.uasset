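; Enemy projectile that flies forward and destroys itself when it overlaps something other than an enemy.
; Tick moves it along its forward vector at Speed without sweeping, so hits rely on actor overlap events.
; Overlaps with BP_EnemyBase actors are ignored; others trigger destruction after a short delay, preceded by an explosion effect and sound unless tagged DeathPlane or PowerUp.
; The Blueprint itself applies no damage.
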(event EventBeginPlay)

(event Collision|EventActorBeginOverlap
  (params (OtherActor :type Actor%20Object%20Reference))
  (bind _tags (Variables|/Script/Engine.Actor|GetTags OtherActor))
  (Utilities|Casting|CastToBP_EnemyBase OtherActor
    (:CastFailed
      (if (or (Utilities|Array|ContainsItem _tags "DeathPlane") (Utilities|Array|ContainsItem _tags "PowerUp"))
        _
        (else
          (Effects|SpawnEmitteratLocation "/Game/StarterContent/Particles/P_Explosion.P_Explosion" (Transformation|GetActorLocation))
          (Audio|PlaySound2D "/Game/StarterContent/Audio/Explosion01.Explosion01" 1.0 1.0 0.0 0 0)))
      (Utilities|FlowControl|Delay 0.2)
      (Actor|DestroyActor))))

(event EventTick
  (params (DeltaSeconds :type Float%20%28single-precision%29))
  (Transformation|SetActorLocation (+ (* (Transformation|GetActorForwardVector) (* DeltaSeconds (Variables|Default|GetSpeed))) (Transformation|GetActorLocation)) false false))

(fn ConstructionScript)