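; BP_EnemyH is an enemy child Blueprint that sets a sideways movement vector along its right axis and reverses it on overlapping wall-tagged actors.
; Each right-to-left turn also shortens the shot delay, clamped to a minimum threshold, while left-to-right turns only flip direction.
; BeginPlay sets initial direction and ammo damage; other overlaps go to the parent, and no movement or firing logic appears here.
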(event EventBeginPlay
  (Variables|Default|SetMovementVector (Transformation|GetActorRightVector))
  (Variables|Default|SetIsRight true)
  (Variables|Default|SetAmmoDamage 2))

(event Collision|EventActorBeginOverlap
  (params (OtherActor :type Actor%20Object%20Reference))
  (bind _returnvalue (Transformation|GetActorRightVector))
  (if (Utilities|Array|ContainsItem (Variables|/Script/Engine.Actor|GetTags OtherActor) (Variables|Default|GetWallTag))
    (if (Variables|Default|GetIsRight)
      (Variables|Default|SetIsRight false)
      (Variables|Default|SetMovementVector (* _returnvalue -1.0))
      (Variables|Default|SetDelayShoot (- (Variables|Default|GetDelayShoot) 0.1))
      ;[0.15 0.15 0.15 0.5] Make sure that Delay Shoot is always >= 0.5
      (if (<= (Variables|Default|GetDelayShoot) (Variables|Default|GetDelayShootThreshold))
        (Variables|Default|SetDelayShoot (Variables|Default|GetDelayShootThreshold)))
      (else
        (Variables|Default|SetIsRight true)
        (Variables|Default|SetMovementVector _returnvalue)))
    (else
      (|CallParentFunction OtherActor))))

(event EventTick
  (params (DeltaSeconds :type Float%20%28single-precision%29))
  (|CallParentFunction DeltaSeconds) ; This node is disabled and will not be called.\nDrag off pins to build functionality.
)

(fn ConstructionScript
  (|CallParentFunction))