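; Enemy generator that spawns random enemies on a looping timer at randomly chosen tagged scene components on itself.
; The game mode's Level sets the random range for picking base, horizontal or patroller enemies, clamped by MaxNumEnemies.
; Each spawned enemy's destroyed event lowers SpawnTime within a clamped range, but the timer set at BeginPlay is never restarted with the new value.
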(event Custom|Spawn
  (bind _enemyspawned (CallFunction|SpawnEnemy))
  (EventDispatchers|BindEventtoOnEnemyDestroy _enemyspawned (delegate Custom|EnemyDestroyed)))

(event Custom|EnemyDestroyed
  (Variables|Default|SetSpawnTime (Math|Float|Clamp(Float) (- (Variables|Default|GetSpawnTime) 0.1) 0.5 2.0)))

(event EventBeginPlay
  (Utilities|Time|SetTimerbyEvent (delegate Custom|Spawn) (Variables|Default|GetSpawnTime) true)
  (bind _asbp_ss_game_mode (Utilities|Casting|CastToBP_SS_GameMode (Game|GetGameMode)))
  (Variables|Default|Set_GameMode _asbp_ss_game_mode))

(event Collision|EventActorBeginOverlap
  (params (OtherActor :type Actor%20Object%20Reference)))

(event EventTick
  (params (DeltaSeconds :type Float%20%28single-precision%29)))

(fn ConstructionScript)

(fn SpawnEnemy
  (bind _spawnpointtag (Variables|Default|GetSpawnPointTag))
  (bind _returnvalue (Actor|GetComponentsbyTag "/Script/Engine.SceneComponent" _spawnpointtag))
  (bind _enemyclass (CallFunction|GetClasstoSpawn (Math|Random|RandomInteger (Variables|/Game/System/BP_SS_GameMode.BP_SS_GameMode_C|GetLevel (Variables|Default|Get_GameMode)))))
  (bind _returnvalue_2 (Game|SpawnActorfromClass _enemyclass (Transformation|GetWorldTransform (Utilities|Array|Get(acopy) _returnvalue (Math|Random|RandomInteger (Utilities|Array|Length _returnvalue)))) "Undefined" "MultiplyWithRoot" 0 0))
  (return _returnvalue_2))

(fn GetClasstoSpawn
  (params (Type :type Integer))
  (return (Utilities|Select :Index (Math|Integer|Clamp(Integer) Type 0 (- (Variables|Default|GetMaxNumEnemies) 1)) :Option%200 "/Game/Enemies/BP_EnemyBase.BP_EnemyBase_C" :Option%201 "/Game/Enemies/BP_EnemyHorizontal.BP_EnemyHorizontal_C" :Option%202 "/Game/Enemies/BP_EnemyPatroller.BP_EnemyPatroller_C")))