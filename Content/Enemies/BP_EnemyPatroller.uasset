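; BP_EnemyPatroller is an enemy that travels along a spline path while firing periodically.
; On BeginPlay it picks a random BP_EnemySpline actor from the level as its path.
; Each Tick it advances a distance by speed and delta time and moves to that world location on the spline, without matching rotation.
; A timer accumulated in Tick calls Fire whenever the shoot delay is exceeded.
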(event EventBeginPlay
  (bind _outactors (Actor|GetAllActorsOfClass "/Game/Enemies/BP_EnemySpline.BP_EnemySpline_C"))
  (Variables|Default|SetSpline (.OutItem (Utilities|Array|Random _outactors))))

(event Collision|EventActorBeginOverlap
  (params (OtherActor :type Actor%20Object%20Reference)))

(event EventTick
  (params (DeltaSeconds :type Float%20%28single-precision%29))
  (bind _output_get (Variables|Default|SetPositionOnSpline (+ (* DeltaSeconds (Variables|Default|GetSpeedOnSpline)) (Variables|Default|GetPositionOnSpline))))
  (Transformation|SetActorLocation (.location (Spline|GetTransformatDistanceAlongSpline (Variables|/Game/Enemies/BP_EnemySpline.BP_EnemySpline_C|GetSpline (Variables|Default|GetSpline)) _output_get "World" false)) false false)
  (bind _output_get_2 (Variables|Default|SetShotCurrentTime (+ DeltaSeconds (Variables|Default|GetShotCurrentTime))))
  (if (> _output_get_2 (Variables|Default|GetDelayShoot))
    (Variables|Default|SetShotCurrentTime 0.0)
    (CallFunction|Fire)))

(fn ConstructionScript
  (|CallParentFunction))