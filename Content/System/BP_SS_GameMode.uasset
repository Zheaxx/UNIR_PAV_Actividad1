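; BP_SS_GameMode is a game mode that relays player status to BP_SS_HUD and tracks kills, level and progress.
; It caches the HUD on BeginPlay, then forwards life, shield and death events as widget updates or dedicated HUD calls.
; Each destroyed enemy recalculates Progress from the total kill count with a level-based multiplier and refreshes the HUD.
; Level rises every second kill, after that recalculation.
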(event Custom|PlayerDead
  (bind __hud (Variables|Default|Get_HUD))
  (Default|PlayerKilled __hud)
  (Default|OnWidgetChanged __hud))

(event Custom|EnemyDestroyed
  (Variables|Default|SetEnemiesDestroyed (+ (Variables|Default|GetEnemiesDestroyed) 1))
  (CallFunction|UpdateProgress)
  (if (== (Math|Integer|%(Integer) (Variables|Default|GetEnemiesDestroyed) 2) 0)
    (Variables|Default|SetLevel (+ (Variables|Default|GetLevel) 1))))

(event Custom|TakeShieldDamage
  (Default|OnWidgetChanged (Variables|Default|Get_HUD)))

(event Custom|ShieldDisabled
  (Default|ShieldDisabled (Variables|Default|Get_HUD)))

(event Custom|ShieldEnabled
  (Default|ShieldEnabled (Variables|Default|Get_HUD)))

(event Custom|TakeLifesDamage
  (Default|OnWidgetChanged (Variables|Default|Get_HUD)))

(event Custom|HealLife
  (Default|OnWidgetChanged (Variables|Default|Get_HUD)))

(event EventBeginPlay
  (bind _asbp_ss_hud (Utilities|Casting|CastToBP_SS_HUD (HUD|GetHUD (Game|GetPlayerController 0))))
  (Variables|Default|Set_HUD _asbp_ss_hud))

(event EventTick
  (params (DeltaSeconds :type Float%20%28single-precision%29)))

(fn ConstructionScript)

(fn UpdateProgress
  (if (< (Variables|Default|GetLevel) 2)
    (Variables|Default|SetProgress (* (Variables|Default|GetEnemiesDestroyed) 100))
    (else
      (Variables|Default|SetProgress (* (Variables|Default|GetEnemiesDestroyed) 300))))
  (Default|OnWidgetChanged (Variables|Default|Get_HUD)))